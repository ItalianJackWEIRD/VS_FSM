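; BP_OverlayTrigger is a box trigger volume that requests a raise on the BreathingComponent of any VS_FSMCharacter entering it.
; On begin overlap it calls RequestRaise, passing RaiseHeight as the target height along with HoldSeconds.
; On end overlap it calls RequestLower, but only when LowerOnExit is set.
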(event OnComponentBeginOverlap(Box)
  (params (OverlappedComponent :type Primitive%20Component%20Object%20Reference) (OtherActor :type Actor%20Object%20Reference) (OtherComp :type Primitive%20Component%20Object%20Reference) (OtherBodyIndex :type Integer) (bFromSweep :type Boolean) (SweepResult :type Hit%20Result%20Structure%20%28by%20ref%29))
  (bind _asvs_fsmcharacter (Utilities|Casting|CastToVS_FSMCharacter OtherActor))
  (Class|BreathingComponent|RequestRaise (Actor|GetComponentbyClass _asvs_fsmcharacter "/Script/VS_FSM.BreathingComponent") (Variables|Default|GetRaise%20Height) (Variables|Default|GetHold%20Seconds)))

(event OnComponentEndOverlap(Box)
  (params (OverlappedComponent :type Primitive%20Component%20Object%20Reference) (OtherActor :type Actor%20Object%20Reference) (OtherComp :type Primitive%20Component%20Object%20Reference) (OtherBodyIndex :type Integer))
  (if (Variables|Default|GetLower%20on%20Exit)
    (bind _asvs_fsmcharacter (Utilities|Casting|CastToVS_FSMCharacter OtherActor))
    (Class|BreathingComponent|RequestLower (Actor|GetComponentbyClass _asvs_fsmcharacter "/Script/VS_FSM.BreathingComponent"))))

(event EventBeginPlay)

(event Collision|EventActorBeginOverlap
  (params (OtherActor :type Actor%20Object%20Reference)))

(event EventTick
  (params (DeltaSeconds :type Float%20%28single-precision%29)))

(fn ConstructionScript)